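; Pistol weapon Blueprint that the player can pick up, built on a parent weapon class.
; On BeginPlay it calls the parent, then sets its defaults as a semi-automatic gun with its clip size, starting ammunition and damage.
; It overrides the interaction text functions to show a pickup prompt attached to the gun mesh.
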(event `self.ReceiveBeginPlay`
  ;[1 1 1] Setting Default Variables
  (`parent.ReceiveBeginPlay`)
  (set `self.bIsAutomatic` false)
  (set `self.Ammunition` 10)
  (set `self.MaxClipSize` 10)
  (set `self.DealDamage` 4))

(fn `GetInteractionText`
  (returns (`Item Text` :type Text))
  (return "Pickup Pistol"))

(fn `GetInteractionTextAttach`
  (returns (AttachComponent :type "SceneComponent Object Reference"))
  (return (`self.GunMesh`)))

(fn `UserConstructionScript`
  (`parent.UserConstructionScript`))