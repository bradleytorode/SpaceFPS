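; Pickup gun actor that the player interacts with to equip, then fires as a hitscan weapon that damages CreatureBase actors.
; Interaction hands it to the character, while SetGunState swaps collision profiles between Dropped and Equipped.
; Shoot line-traces from the muzzle to the player owner's scaled forward vector, without adding the start position, drawing persistent debug lines.
; Drop only resets state, as physics simulation is unused.
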(event `Shoot`
  (bind _outhit (`KismetSystemLibrary.LineTraceSingle` :`Start` (`SceneComponent.GetSocketLocation` (`self.GunMesh`) "Muzzle") :`End` (* (`self.GetActorForwardVector` (`self.GetOwner` (`GameplayStatics.GetPlayerCharacter` 0))) 10000.0) :`TraceChannel` "TraceTypeQuery1" :`bTraceComplex` true :`DrawDebugType` "Persistent"))
  (bind (_bblockinghit _binitialoverlap _time _distance _location _impactpoint _normal _impactnormal _physmat _hitactor) (`GameplayStatics.BreakHitResult` _outhit))
  (if _bblockinghit
    (bind _ascreature_base (cast `CreatureBase` _hitactor))
    (`CreatureBase.TakeDamage` _ascreature_base (`self.DealDamage`))))

(event `self.ReceiveBeginPlay`
  (`self.SetGunState` "NewEnumerator0"))

(event `/Game/BradleyFiles/Items/InteractionInterface/InteractionInterface.OnInteracted`
  (params (Character :type "/Game/BradleyFiles/Character/BradPlayerCharacter_BP Object Reference"))
  (`/Game/BradleyFiles/Character/BradPlayerCharacter_BP.Pick Up Gun` Character self)
  (`self.SetGunState` "NewEnumerator1"))

(fn `Drop`
  ;[1 1 1] Redundant Code. It can't simulate Physics
  (`self.SetGunState` "NewEnumerator0"))

(fn `GetInteractionText`
  (returns (`Item Text` :type Text))
  (return (`KismetTextLibrary.Conv_StringToText` (`KismetStringLibrary.Concat_StrStr` " Pickup: " "Gun"))))

(fn `GetInteractionTextAttach`
  (returns (AttachComponent :type "SceneComponent Object Reference"))
  (return (`self.GunMesh`)))

(fn `SetGunState`
  (params (`New Gun State` :type "/Game/BradleyFiles/Items/WeaponBPs/E_GunState Enum" :default "NewEnumerator0"))
  (bind _gunmesh (`self.GunMesh`))
  (bind _output_get (set `self.GunState` `New Gun State`))
  (switch `/Game/BradleyFiles/Items/WeaponBPs/E_GunState` _output_get
    (:`NewEnumerator0`
      (`PrimitiveComponent.SetCollisionProfileName` (`self.Sphere`) "OverlapAllDynamic" true)
      (`PrimitiveComponent.SetCollisionProfileName` (`self.GunMesh`) "DroppedGun" true))
    (:`NewEnumerator1`
      (`PrimitiveComponent.SetCollisionProfileName` (`self.Sphere`) "NoCollision" true)
      (`PrimitiveComponent.SetCollisionProfileName` _gunmesh "NoCollision" true)
      (`SceneComponent.ResetRelativeTransform` _gunmesh))))

(fn `UserConstructionScript`
  (`parent.UserConstructionScript`))