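; BP_ItemBase is a base item Blueprint that shows an interaction prompt while a character is in range.
; On range entry it creates a screen-space, collision-free widget component at runtime, guarded against duplicates, and destroys it on exit.
; The prompt text and attach component come from GetInteractionText and GetInteractionTextAttach, which default to "Interact" and the scene root for child classes to override.
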(event `/Game/BradleyFiles/Items/InteractionInterface/InteractionInterface.OnInteractionRangeEntered`
  (params (Character :type "/Game/BradleyFiles/Character/BradPlayerCharacter_BP Object Reference"))
  ;[1 1 1] Add Widget to the screen and change Text accordingly dependent on the item that is created
  ;;[1 1 1] Check to make sure interaction widget isn't created twice on accident
  (`self.InteractionWidgetComponent`
    (:`then`)
    (:`else`
      (bind _returnvalue (`|CreateWidget` "/Game/BradleyFiles/Items/InteractionInterface/InteractionWidget.InteractionWidget_C" (cast `PlayerController` (`Pawn.GetController` Character) :!pure true) (`self.GetInteractionText`)))
      (bind _returnvalue_2 (`AddComponent|NODE_AddWidgetComponent-0`))
      ;;[1 1 1] Set Interaction for deletion on interaction range exited
      (bind _output_get (set `self.InteractionWidgetComponent` _returnvalue_2))
      ;;[1 1 1] Set Widget to the size of the size box created in the widget blueprint and draw it making sure the player/item wont collide with the text.
      (`WidgetComponent.SetWidget` _output_get _returnvalue)
      ;;;[1 1 1] Visible no matter where player walks
      (`WidgetComponent.SetWidgetSpace` _output_get "Screen")
      (`WidgetComponent.SetDrawAtDesiredSize` _output_get true)
      (`PrimitiveComponent.SetCollisionEnabled` _output_get "NoCollision")
      (`SceneComponent.K2_AttachToComponent` _output_get (`self.GetInteractionTextAttach`) "None" "SnapToTarget" "SnapToTarget" "SnapToTarget" true))))

(event `/Game/BradleyFiles/Items/InteractionInterface/InteractionInterface.OnInteractionRangeExited`
  ;[1 1 1] If the interaction range is valid and been exited, then destroy the text component.
  (bind _interactionwidgetcomponent (`self.InteractionWidgetComponent`)
    (:`then`
      (`ActorComponent.K2_DestroyComponent` _interactionwidgetcomponent))
    (:`else`)))

(fn `GetInteractionText`
  (returns (`Item Text` :type Text))
  ;[1 1 1] Default Text. To be changed in child classes.
  (return "Interact"))

(fn `GetInteractionTextAttach`
  (returns (AttachComponent :type "SceneComponent Object Reference"))
  ;[1 1 1] What Parent to attach to.
  (return (`self.DefaultSceneRoot`)))

(fn `UserConstructionScript`)