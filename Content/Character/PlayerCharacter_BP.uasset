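; Player character Blueprint that handles item pickup, inventory display, XP gain and heart-based health display.
; Each Tick it polls the capsule for overlapping item actors, adds their class to the inventory and destroys them.
; The inventory is a widget created on BeginPlay and shown by ToggleInventory, while X grants fixed XP through LevelingSystem.
; ModifyHealth steps MainHUD hearts one point at a time, looking up the widget by class each step.
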(event `self.ReceiveTick`
  (params (DeltaSeconds :type "Float (single-precision)"))
  ;[1 1 1] Confirms Collision with other actors and destroys actor
  (for _array_element (`PrimitiveComponent.GetOverlappingActors` (`self.CapsuleComponent`) "/Game/AkiraStuff/Items/BP_ItemBaseC.BP_ItemBaseC_C")
    (`/Game/AkiraStuff/UI/Widgets/InventoryUI/InventoryWidget.AddItem` (`self.Inventory`) (castclass `/Game/AkiraStuff/Items/BP_ItemBaseC` (`GameplayStatics.GetObjectClass` _array_element) :!pure true))
    (`self.K2_DestroyActor` _array_element)))

(event `Key|X`
  (params (Key :type "Key Structure"))
  ;[1 1 1] Adds XP when x is pressed
  (:`Pressed`
    (`/Game/AkiraStuff/LevelingSystem/LevelingSystem.AddXP` (`self.LevelingSystem`) 200.0)))

(event `self.ReceiveBeginPlay`
  ;[1 1 1] Makes the inventory exists
  (bind _returnvalue (`|CreateWidget` "/Game/AkiraStuff/UI/Widgets/InventoryUI/InventoryWidget.InventoryWidget_C" (`GameplayStatics.GetPlayerController` 0)))
  (set `self.Inventory` _returnvalue))

(event `InputAction|ToggleInventory`
  (params (Key :type "Key Structure"))
  (:`Pressed`
    (if (not (`Widget.IsInViewport` (`self.Inventory`)))
      (`/Game/AkiraStuff/UI/Widgets/InventoryUI/InventoryWidget.Show` (`self.Inventory`) Key))))

(fn `ModifyHealth`
  (params (HealthAmount :type Integer))
  ;[1 1 1] Adjusts the health
  (if (>= HealthAmount 0)
    (for _ (range HealthAmount)
      (bind _foundwidgets (`WidgetBlueprintLibrary.GetAllWidgetsOfClass` "/Game/AkiraStuff/UI/MainHud.MainHUD_C"))
      (`/Game/AkiraStuff/UI/MainHud.UpdateHearts` (`|GetArrayItem` _foundwidgets) 1))
    (else
      (for _ (range (* HealthAmount -1))
        (bind _foundwidgets_2 (`WidgetBlueprintLibrary.GetAllWidgetsOfClass` "/Game/AkiraStuff/UI/MainHud.MainHUD_C"))
        (`/Game/AkiraStuff/UI/MainHud.UpdateHearts` (`|GetArrayItem` _foundwidgets_2) -1)))))

(fn `UserConstructionScript`)